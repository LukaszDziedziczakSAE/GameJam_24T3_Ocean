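; Game mode Blueprint that handles starting a game and the player's death.
; PlayerStartGame flags BP_GameState as running and started, then has BP_HUD show the game HUD.
; PlayerDied shows the end screen through BP_HUD, clears the game state's running flag and prints a debug message.
; Both functions fetch the HUD from player controller 0, and the event graph holds only disabled default events.
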(event EventBeginPlay)

(event EventTick
  (params (DeltaSeconds :type Float%20%28single-precision%29)))

(fn ConstructionScript)

(fn PlayerDied
  (bind _asbp_hud (Utilities|Casting|CastToBP_HUD (HUD|GetHUD (Game|GetPlayerController 0))))
  (Class|OceanHUD|ShowEndScreen _asbp_hud)
  (bind _asbp_game_state (Utilities|Casting|CastToBP_GameState (Game|GetGameState)))
  (Variables|/Game/Blueprints/BP_GameState.BP_GameState_C|SetGame%20Running _asbp_game_state false)
  (Development|PrintString "Player died"))

(fn PlayerStartGame
  (bind _asbp_game_state (Utilities|Casting|CastToBP_GameState (Game|GetGameState)))
  (Variables|/Game/Blueprints/BP_GameState.BP_GameState_C|SetGame%20Running _asbp_game_state true)
  (Variables|/Game/Blueprints/BP_GameState.BP_GameState_C|SetGame%20Started _asbp_game_state true)
  (bind _asbp_hud (Utilities|Casting|CastToBP_HUD (HUD|GetHUD (Game|GetPlayerController 0))))
  (Class|OceanHUD|ShowGameHUD _asbp_hud))