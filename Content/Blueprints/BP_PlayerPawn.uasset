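; BP_PlayerPawn is the player pawn, and its graph drives breathing and choking audio from the state of its air system.
; Each Tick it polls BPAirSystem, choosing breathing while air recharges and choking when air runs low, and stopping audio otherwise.
; A single AudioComponent plays both sounds and only takes a new one when inactive, so a playing sound is not swapped directly.
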(event EventBeginPlay)

(event Collision|EventActorBeginOverlap
  (params (OtherActor :type Actor%20Object%20Reference)))

(event EventTick
  (params (DeltaSeconds :type Float%20%28single-precision%29))
  (bind _bp_airsystem (Variables|Default|GetBP_AirSystem))
  (bind _audiocomponent (Variables|Default|GetAudioComponent))
  (bind _returnvalue (Components|Activation|IsActive _audiocomponent))
  (if (Variables|/Game/Blueprints/BP_AirSystem.BP_AirSystem_C|GetbRecharging _bp_airsystem)
    (if (not _returnvalue)
      (Audio|Components|Audio|SetSound _audiocomponent (Variables|Default|GetBreathingSound))
      (Audio|Components|Audio|Play _audiocomponent 0.0))
    (elif (< (Default|AirPercentage _bp_airsystem) 0.2)
      (if (not _returnvalue)
        (Audio|Components|Audio|SetSound _audiocomponent (Variables|Default|GetChockingSound))
        (Audio|Components|Audio|Play _audiocomponent 0.0))
      (elif _returnvalue
        (Audio|Components|Audio|Stop _audiocomponent)))))

(fn ConstructionScript)