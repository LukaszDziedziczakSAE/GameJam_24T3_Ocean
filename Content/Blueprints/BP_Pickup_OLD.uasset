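; Collectible pickup actor that counts itself toward the player's collection when touched.
; When a BP_PlayerPawn overlaps its Sphere, it increments Collected on that pawn's CollectiblesSystem and destroys itself.
; It enables input for player controller 0 on BeginPlay but handles no input events.
; The end-overlap handler only casts, and a debug print is left unconnected.
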(event OnComponentBeginOverlap(Sphere)
  (params (OverlappedComponent :type Primitive%20Component%20Object%20Reference) (OtherActor :type Actor%20Object%20Reference) (OtherComp :type Primitive%20Component%20Object%20Reference) (OtherBodyIndex :type Integer) (bFromSweep :type Boolean) (SweepResult :type Hit%20Result%20Structure%20%28by%20ref%29))
  (bind _asbp_player_pawn (Utilities|Casting|CastToBP_PlayerPawn OtherActor))
  (bind _result (Math|Integer|IncrementInt (Variables|/Game/Blueprints/BP_Collectibles.BP_Collectibles_C|GetCollected (Variables|/Game/Blueprints/BP_PlayerPawn.BP_PlayerPawn_C|GetCollectibles%20System _asbp_player_pawn)))
    (:%20%20
      (Variables|/Game/Blueprints/BP_Collectibles.BP_Collectibles_C|SetCollected (Variables|/Game/Blueprints/BP_PlayerPawn.BP_PlayerPawn_C|GetCollectibles%20System _asbp_player_pawn) _result)
      (Actor|DestroyActor))))

(event OnComponentEndOverlap(Sphere)
  (params (OverlappedComponent :type Primitive%20Component%20Object%20Reference) (OtherActor :type Actor%20Object%20Reference) (OtherComp :type Primitive%20Component%20Object%20Reference) (OtherBodyIndex :type Integer))
  (Utilities|Casting|CastToBP_PlayerPawn OtherActor))

(event EventTick
  (params (DeltaSeconds :type Float%20%28single-precision%29)))

(event EventBeginPlay
  (Input|EnableInput (Game|GetPlayerController 0)))

(event Input|KeyboardEvents|F
  (params (Key :type Key%20Structure)))

(fn ConstructionScript)