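; BP_AirSystem is a component on the player pawn that manages the air supply and ends the game when it runs out.
; While the game instance reports the game running, Tick refills air when Recharging and otherwise drains it, calling EndGame on the game mode at zero.
; An upgrade event from PlayerInteractionComponent advances an index into MaxAirLevels to change capacity.
; HasAir and AirPercentage expose the current state.
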(event Custom|UpgraddeMaxAirLevel
  (bind _output_get (Variables|Default|SetCurrentAirLevel (+ (Variables|Default|GetCurrentAirLevel) 1)))
  (Variables|Default|SetMaxAirLevel (Utilities|Array|Get(acopy) (Variables|Default|GetMaxAirLevels) _output_get)))

(event EventBeginPlay
  (Variables|Default|SetAirLevel (Variables|Default|GetMaxAirLevel))
  (bind _asbp_game_instance (Utilities|Casting|CastToBP_GameInstance (Game|GetGameInstance)))
  (Variables|Default|SetGame%20Instance _asbp_game_instance)
  (bind _asbp_player_pawn (Utilities|Casting|CastToBP_PlayerPawn (Components|GetOwner)))
  (EventDispatchers|BindEventtoUpgradeAirLevel (Variables|/Script/GameJam_24T3_Ocean.PlayerPawn|GetPlayerInteractionComponent _asbp_player_pawn) (delegate Custom|UpgraddeMaxAirLevel)))

(event EventTick
  (params (DeltaSeconds :type Float%20%28single-precision%29))
  (bind _game_instance (Variables|Default|GetGame%20Instance)
    (:then
      (if (Variables|/Game/Blueprints/BP_GameInstance.BP_GameInstance_C|GetGame%20Running _game_instance)
        (if (Variables|Default|GetbRecharging)
          (Variables|Default|SetAirLevel (Math|Float|Clamp(Float) (+ (Variables|Default|GetAirLevel) (* (Variables|Default|GetAirRefillRate) DeltaSeconds)) 0.0 (Variables|Default|GetMaxAirLevel)))
          (elif (CallFunction|HasAir)
            (Variables|Default|SetAirLevel (Math|Float|Clamp(Float) (- (Variables|Default|GetAirLevel) (* (Variables|Default|GetAirConsumptionRate) DeltaSeconds)) 0.0 (Variables|Default|GetMaxAirLevel)))
            (else
              (bind _asbp_game_mode (Utilities|Casting|CastToBP_GameMode (Game|GetGameMode)))
              (Class|OceanGameMode|EndGame _asbp_game_mode))))))
    (:else)))

(fn AirConsumption)

(fn HasAir
  (return (> (Variables|Default|GetAirLevel) 0.0)))

(fn AirPercentage
  (return (/ (Variables|Default|GetAirLevel) (Variables|Default|GetMaxAirLevel))))