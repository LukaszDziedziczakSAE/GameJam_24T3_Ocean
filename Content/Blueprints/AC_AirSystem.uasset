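; AC_AirSystem is an unfinished air supply system with an air level and a consumption rate.
; BeginPlay and Tick are empty, and a disconnected graph copy of the depletion check never runs.
; The AirConsumption function repeats that check with zero delta time and an empty branch, never updating AirLevel.
; HasAir is true when the computed level falls below zero, the opposite of its name.
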(event EventBeginPlay)

(event EventTick
  (params (DeltaSeconds :type Float%20%28single-precision%29)))

(fn AirConsumption
  (bind _output_get (Variables|Default|SetHasAir (< (- (Variables|Default|GetAirLevel) (* (Variables|Default|GetAirConsumptionRate) 0.0)) 0.0)))
  (if _output_get
    _))